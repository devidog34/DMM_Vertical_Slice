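; BP_HealthPickup is a collectible that restores a small, fixed amount of the player's health on contact.
; When its Box component is overlapped by a BP_MainPlayer, it raises CurrentHealth, clamps it to a hardcoded range and destroys itself.
; The pickup is consumed even at full health, and other actors are ignored.
; An unconnected variant targeting BP_ThirdPersonCharacter with a larger heal remains in the graph and never runs.
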(event OnComponentBeginOverlap(Box)
  (params (OverlappedComponent :type Primitive%20Component%20Object%20Reference) (OtherActor :type Actor%20Object%20Reference) (OtherComp :type Primitive%20Component%20Object%20Reference) (OtherBodyIndex :type Integer) (bFromSweep :type Boolean) (SweepResult :type Hit%20Result%20Structure%20%28by%20ref%29))
  (bind _asbp_main_player (Utilities|Casting|CastToBP_MainPlayer OtherActor))
  (Variables|/Game/DavidsMightyMen/Core/DamageSystem/BP_MainPlayer.BP_MainPlayer_C|SetCurrent%20Health _asbp_main_player (Math|Float|Clamp(Float) (+ (Variables|/Game/DavidsMightyMen/Core/DamageSystem/BP_MainPlayer.BP_MainPlayer_C|GetCurrent%20Health _asbp_main_player) 1e+01) 0.0 1e+02))
  (Actor|DestroyActor))

(event EventBeginPlay)

(event Collision|EventActorBeginOverlap
  (params (OtherActor :type Actor%20Object%20Reference)))

(event EventTick
  (params (DeltaSeconds :type Float%20%28single-precision%29)))

(fn ConstructionScript)