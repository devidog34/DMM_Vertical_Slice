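; BP_Enemy_Melee is a melee enemy Blueprint that implements sword equip, unequip and attack events.
; Equipping spawns BP_Weapon_Sword and snaps it to the right-hand socket on the mesh, while unequipping destroys it, both updating the wielding flag.
; Attack calls a montage node with no montage assigned, signalling attack end with a debug print immediately, as well as on completion or interruption.
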(event EventEquipWeapon
  (Default|CallOnEquipWeapon)
  (bind _returnvalue (Game|SpawnActorfromClass "/Game/DavidsMightyMen/Core/Weapons/BP_Weapon_Sword.BP_Weapon_Sword_C" (Transformation|GetActorTransform) "Undefined" "MultiplyWithRoot" 0 0))
  (bind _output_get (Variables|Default|SetWeaponActor _returnvalue))
  (Transformation|AttachComponentToComponent _output_get (Variables|Character|GetMesh) "hand_r_sword_socket" "SnapToTarget" "SnapToTarget" "SnapToTarget" true)
  (Variables|Default|SetIsWieldingWeapon true))

(event EventUnequipWeapon
  (Actor|DestroyActor (Variables|Default|GetWeaponActor))
  (Variables|Default|SetIsWieldingWeapon false)
  (Default|CallOnUnequipWeapon))

(event EventAttack
  (Animation|Montage|PlayMontage (Variables|Character|GetMesh) 0
    (:then
      _)
    (:OnCompleted
      _)
    (:OnInterrupted
      _))
  (Default|CallOnAttackEnd)
  (Development|PrintString "Enemy Attacked"))

(fn ConstructionScript
  (|CallParentFunction))